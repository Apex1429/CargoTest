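; Player controller Blueprint that sets up mouse-driven input and an on-screen test UI.
; BeginPlay enables click events, shows the cursor, then creates a WidgetTest widget and adds it to the viewport.
; Currency, DataRef, GameInstanceRef and StatStruct are empty stubs: Currency returns zero and the others return without doing any work.
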(event `self.ReceiveBeginPlay`
  (set `self.bEnableClickEvents` true)
  (set `self.bShowMouseCursor` true)
  (bind _returnvalue (`|CreateWidget` "/Game/UserInterface/WidgetTest.WidgetTest_C"))
  (`UserWidget.AddToViewport` _returnvalue 0))

(fn `Currency`
  (params (Player :type "GameInstance Object Reference"))
  (returns (Currency :type Integer))
  (return 0))

(fn `DataRef`
  (returns (LocationStuff :type "/Game/Data/LocationStruct Structure"))
  (return))

(fn `GameInstanceRef`
  (returns (PlayerRef :type "/Game/BP_GameInstance Object Reference"))
  (return null))

(fn `StatStruct`
  (params (ChangeStats :type "/Game/Data/PlayerStats_Struct Structure"))
  (returns (Stats :type "/Game/Data/PlayerStats_Struct Structure"))
  (return))

(fn `UserConstructionScript`)